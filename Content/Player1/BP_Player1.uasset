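; Player 1 character Blueprint that handles Enhanced Input movement, camera look and montage-driven combat moves.
; On possession it adds IMC_Player; move actions follow control yaw, scaled by a Speed value that Left Shift toggles via FlipFlop.
; Mouse buttons and number keys play kick, punch and down montages directly on the mesh.
; Jump likewise only plays a montage, with no Character Jump call.
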(event `self.ReceivePossessed`
  (params (NewController :type "Controller Object Reference"))
  (bind _asplayer_controller (cast `PlayerController` NewController))
  (message `EnhancedInputSubsystemInterface.AddMappingContext` (pcsubsystem `EnhancedInputLocalPlayerSubsystem` _asplayer_controller) "/Game/input/IMC_Player.IMC_Player" 0 (struct)))

(event `EnhancedInput|/Game/input/IA_Jump`
  (params (ActionValue :type Boolean) (ElapsedSeconds :type "Float (double-precision)") (TriggeredSeconds :type "Float (double-precision)") (InputAction :type "InputAction Object Reference" :default "/Game/input/IA_Jump.IA_Jump"))
  (:`Triggered`
    (`|PlayMontage` (`self.Mesh`) "/Game/Player1/Animations/P1Jump1_MTG.P1Jump1_MTG")))

(event `EnhancedInput|/Game/input/IA_Turn`
  (params (ActionValue :type "Float (double-precision)") (ElapsedSeconds :type "Float (double-precision)") (TriggeredSeconds :type "Float (double-precision)") (InputAction :type "InputAction Object Reference" :default "/Game/input/IA_Turn.IA_Turn"))
  (:`Triggered`
    (`self.AddControllerYawInput` ActionValue)))

(event `EnhancedInput|/Game/input/IA_MouseL`
  (params (ActionValue :type Boolean) (ElapsedSeconds :type "Float (double-precision)") (TriggeredSeconds :type "Float (double-precision)") (InputAction :type "InputAction Object Reference" :default "/Game/input/IA_MouseL.IA_MouseL"))
  (:`Triggered`
    (`|PlayMontage` (`self.Mesh`) "/Game/Player1/Animations/P1Kick1_MTG.P1Kick1_MTG")))

(event `EnhancedInput|/Game/input/IA_LookUp`
  (params (ActionValue :type "Float (double-precision)") (ElapsedSeconds :type "Float (double-precision)") (TriggeredSeconds :type "Float (double-precision)") (InputAction :type "InputAction Object Reference" :default "/Game/input/IA_LookUp.IA_LookUp"))
  (:`Triggered`
    (`self.AddControllerPitchInput` ActionValue)))

(event `EnhancedInput|/Game/input/IA_WS`
  (params (ActionValue :type "Float (double-precision)") (ElapsedSeconds :type "Float (double-precision)") (TriggeredSeconds :type "Float (double-precision)") (InputAction :type "InputAction Object Reference" :default "/Game/input/IA_WS.IA_WS"))
  (bind (_returnvalue_roll _returnvalue_pitch _returnvalue_yaw) (`KismetMathLibrary.BreakRotator` (`self.GetControlRotation`)))
  (:`Triggered`
    (`self.AddMovementInput` (`KismetMathLibrary.GetForwardVector` (`KismetMathLibrary.MakeRotator` 0.0 0.0 _returnvalue_yaw)) (* ActionValue (`self.speed`)))))

(event `EnhancedInput|/Game/input/IA_MouseR`
  (params (ActionValue :type Boolean) (ElapsedSeconds :type "Float (double-precision)") (TriggeredSeconds :type "Float (double-precision)") (InputAction :type "InputAction Object Reference" :default "/Game/input/IA_MouseR.IA_MouseR"))
  (:`Triggered`
    (`|PlayMontage` (`self.Mesh`) "/Game/Player1/Animations/P1Punching1_MTG.P1Punching1_MTG")))

(event `EnhancedInput|/Game/input/IA_1`
  (params (ActionValue :type Boolean) (ElapsedSeconds :type "Float (double-precision)") (TriggeredSeconds :type "Float (double-precision)") (InputAction :type "InputAction Object Reference" :default "/Game/input/IA_1.IA_1"))
  (:`Triggered`
    (`|PlayMontage` (`self.Mesh`) "/Game/Player1/Animations/P1Kick2_MTG.P1Kick2_MTG")))

(event `EnhancedInput|/Game/input/IA_AD`
  (params (ActionValue :type "Float (double-precision)") (ElapsedSeconds :type "Float (double-precision)") (TriggeredSeconds :type "Float (double-precision)") (InputAction :type "InputAction Object Reference" :default "/Game/input/IA_AD.IA_AD"))
  (bind (_returnvalue_roll _returnvalue_pitch _returnvalue_yaw) (`KismetMathLibrary.BreakRotator` (`self.GetControlRotation`)))
  (:`Triggered`
    (`self.AddMovementInput` (`KismetMathLibrary.GetRightVector` (`KismetMathLibrary.MakeRotator` 0.0 0.0 _returnvalue_yaw)) (* ActionValue (`self.speed`)))))

(event `EnhancedInput|/Game/input/IA_2`
  (params (ActionValue :type Boolean) (ElapsedSeconds :type "Float (double-precision)") (TriggeredSeconds :type "Float (double-precision)") (InputAction :type "InputAction Object Reference" :default "/Game/input/IA_2.IA_2"))
  (:`Triggered`
    (`|PlayMontage` (`self.Mesh`) "/Game/Player1/Animations/P1Punching2_MTG.P1Punching2_MTG")))

(event `Key|LeftShift`
  (params (Key :type "Key Structure"))
  (:`Pressed`
    (`/Engine/EditorBlueprintResources/StandardMacros.FlipFlop`
      (:`A`
        (set `self.speed` 0.5))
      (:`B`
        (set `self.speed` 1.0)))))

(event `EnhancedInput|/Game/input/IA_3`
  (params (ActionValue :type Boolean) (ElapsedSeconds :type "Float (double-precision)") (TriggeredSeconds :type "Float (double-precision)") (InputAction :type "InputAction Object Reference" :default "/Game/input/IA_3.IA_3"))
  (:`Triggered`
    (`|PlayMontage` (`self.Mesh`) "/Game/Player1/Animations/P1Down2_MTG.P1Down2_MTG")))

(fn `UserConstructionScript`)