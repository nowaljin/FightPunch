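; BP_Samurai is a playable katana fighter that maps Enhanced Input to attack, jump, sit and death montages, plus camera pitch and single-axis movement with a Shift speed toggle.
; Each Tick, unless AttackFlag is set, it takes its yaw from BattleGameMode's Z1 or Z2 according to PlayerRLNo.
; KatanaON/OFF toggle blade collision, whose overlap calls DamageEvent on BP_Player2 only.
; Its own DamageEvent plays a death montage and spawns a Niagara effect.
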(event `self.ReceiveTick`
  (params (DeltaSeconds :type "Float (single-precision)"))
  ; target Lock
  (`self.Rotation_CHG_Func`))

(event `EnhancedInput|/Game/Input/IA_MouseL`
  (params (ActionValue :type Boolean) (ElapsedSeconds :type "Float (double-precision)") (TriggeredSeconds :type "Float (double-precision)") (InputAction :type "InputAction Object Reference" :default "/Game/Input/IA_MouseL.IA_MouseL"))
  (:`Triggered`
    (`|PlayMontage` (`self.Mesh`) "/Game/Player/Animations/P2ShieldAttack1_MTG.P2ShieldAttack1_MTG")))

(event `self.ReceivePossessed`
  (params (NewController :type "Controller Object Reference"))
  (bind _asplayer_controller (cast `PlayerController` NewController))
  (message `EnhancedInputSubsystemInterface.AddMappingContext` (pcsubsystem `EnhancedInputLocalPlayerSubsystem` _asplayer_controller) "/Game/Input/IMC_Player.IMC_Player" 0 (struct)))

(event `EnhancedInput|/Game/Input/IA_MouseR`
  (params (ActionValue :type Boolean) (ElapsedSeconds :type "Float (double-precision)") (TriggeredSeconds :type "Float (double-precision)") (InputAction :type "InputAction Object Reference" :default "/Game/Input/IA_MouseR.IA_MouseR"))
  (:`Triggered`
    (`|PlayMontage` (`self.Mesh`) "/Game/Player/Animations/P2ShieldAttack3_MTG.P2ShieldAttack3_MTG")))

(event `EnhancedInput|/Game/Input/IA_MouseC`
  (params (ActionValue :type Boolean) (ElapsedSeconds :type "Float (double-precision)") (TriggeredSeconds :type "Float (double-precision)") (InputAction :type "InputAction Object Reference" :default "/Game/Input/IA_MouseC.IA_MouseC"))
  (:`Triggered`
    (`|PlayMontage` (`self.Mesh`) "/Game/Player/Animations/P2Jump_MTG.P2Jump_MTG")))

(event `EnhancedInput|/Game/Input/IA_jump`
  (params (ActionValue :type Boolean) (ElapsedSeconds :type "Float (double-precision)") (TriggeredSeconds :type "Float (double-precision)") (InputAction :type "InputAction Object Reference" :default "/Game/Input/IA_jump.IA_jump"))
  ; Bu Playmontaji eklersen degisik bir jamp update oluyor
)

(event `EnhancedInput|/Game/Input/IA_W`
  (params (ActionValue :type Boolean) (ElapsedSeconds :type "Float (double-precision)") (TriggeredSeconds :type "Float (double-precision)") (InputAction :type "InputAction Object Reference" :default "/Game/Input/IA_W.IA_W"))
  ; Bu Playmontaji eklersen degisik bir jamp update oluyor
  (:`Triggered`
    (`self.Jump`)))

(event `EnhancedInput|/Game/Input/IAKey4`
  (params (ActionValue :type Boolean) (ElapsedSeconds :type "Float (double-precision)") (TriggeredSeconds :type "Float (double-precision)") (InputAction :type "InputAction Object Reference" :default "/Game/Input/IAKey4.IAKey4"))
  ; Bu Playmontaji eklersen degisik bir jamp update oluyor
  (:`Triggered`
    (`self.Jump`)
    (`|PlayMontage` (`self.Mesh`) "/Game/Player/Animations/P2Jump_MTG.P2Jump_MTG")))

(event `EnhancedInput|/Game/Input/IAKey1`
  (params (ActionValue :type Boolean) (ElapsedSeconds :type "Float (double-precision)") (TriggeredSeconds :type "Float (double-precision)") (InputAction :type "InputAction Object Reference" :default "/Game/Input/IAKey1.IAKey1"))
  (:`Triggered`
    (`|PlayMontage` (`self.Mesh`) "/Game/Player2/Animations/deathmon.deathmon" 0.3)))

(event `EnhancedInput|/Game/Input/IA_S`
  (params (ActionValue :type Boolean) (ElapsedSeconds :type "Float (double-precision)") (TriggeredSeconds :type "Float (double-precision)") (InputAction :type "InputAction Object Reference" :default "/Game/Input/IA_S.IA_S"))
  (:`Triggered`
    (`|PlayMontage` (`self.Mesh`) "/Game/Player/Animations/Sit_MTG.Sit_MTG" 1.5)))

(event `KatanaON`
  (`PrimitiveComponent.SetCollisionEnabled` (`self.KatanaBox`) "QueryAndPhysics"))

(event `KatanaOFF`
  (`PrimitiveComponent.SetCollisionEnabled` (`self.KatanaBox`) "NoCollision"))

(event `EnhancedInput|/Game/Input/IA_Turn`
  (params (ActionValue :type "Float (double-precision)") (ElapsedSeconds :type "Float (double-precision)") (TriggeredSeconds :type "Float (double-precision)") (InputAction :type "InputAction Object Reference" :default "/Game/Input/IA_Turn.IA_Turn"))
  ; Mause Movement
)

(event `EnhancedInput|/Game/Input/IA_LookUp`
  (params (ActionValue :type "Float (double-precision)") (ElapsedSeconds :type "Float (double-precision)") (TriggeredSeconds :type "Float (double-precision)") (InputAction :type "InputAction Object Reference" :default "/Game/Input/IA_LookUp.IA_LookUp"))
  (:`Triggered`
    (`self.AddControllerPitchInput` ActionValue)))

(event `ActionON`
  ; Action ON OFF
  (set `self.ActionFlag` true))

(event `EnhancedInput|/Game/Input/IA_WS`
  (params (ActionValue :type "Float (double-precision)") (ElapsedSeconds :type "Float (double-precision)") (TriggeredSeconds :type "Float (double-precision)") (InputAction :type "InputAction Object Reference" :default "/Game/Input/IA_WS.IA_WS")))

(event `ActionOFF`
  ; Action ON OFF
  (set `self.ActionFlag` false))

(event `EnhancedInput|/Game/Input/IA_AD`
  (params (ActionValue :type "Float (double-precision)") (ElapsedSeconds :type "Float (double-precision)") (TriggeredSeconds :type "Float (double-precision)") (InputAction :type "InputAction Object Reference" :default "/Game/Input/IA_AD.IA_AD"))
  (bind (_returnvalue_roll _returnvalue_pitch _returnvalue_yaw) (`KismetMathLibrary.BreakRotator` (`self.GetControlRotation`)))
  (:`Triggered`
    (`self.AddMovementInput` (`KismetMathLibrary.GetForwardVector` (`KismetMathLibrary.MakeRotator` 0.0 0.0 _returnvalue_yaw)) (* ActionValue (`self.speed`)))))

(event `Key|LeftShift`
  (params (Key :type "Key Structure"))
  (:`Pressed`
    (`/Engine/EditorBlueprintResources/StandardMacros.FlipFlop`
      (:`A`
        (set `self.speed` 0.5))
      (:`B`
        (set `self.speed` 1.0)))))

(event `DamageEvent`
  (bind _bodybox (`self.BodyBox`))
  (`self.PlayAnimMontage` "/Game/Player2/Animations/deathmon.deathmon")
  (`NiagaraFunctionLibrary.SpawnSystemAtLocation` "/Game/Free_Spells/VFX_Niagara/NS_Free_Spells_Buff_Mana.NS_Free_Spells_Buff_Mana" (`SceneComponent.K2_GetComponentLocation` _bodybox) (`SceneComponent.K2_GetComponentRotation` _bodybox)))

(event `self.KatanaBox.OnComponentBeginOverlap`
  (params (OverlappedComponent :type "PrimitiveComponent Object Reference") (OtherActor :type "Actor Object Reference") (OtherComp :type "PrimitiveComponent Object Reference") (OtherBodyIndex :type Integer) (bFromSweep :type Boolean) (SweepResult :type "HitResult Structure (by ref)"))
  ; Damage Changer
  (bind _asbp_player_2 (cast `/Game/Player2/BP_Player2` OtherActor))
  (`/Game/Player2/BP_Player2.DamageEvent` _asbp_player_2))

(fn `Rotation_CHG_Func`
  (if (not (`self.attackFlag`))
    (bind _asbattle_game_mode (cast `/Game/Map/BattleGameMode` (`GameplayStatics.GetGameMode`)))
    (if (== (`self.PlayerRL_No`) 0)
      (set `self.zRotation` (`/Game/Map/BattleGameMode.Z1` _asbattle_game_mode))
      (else
        (set `self.zRotation` (`/Game/Map/BattleGameMode.Z2` _asbattle_game_mode))))
    (`self.K2_SetActorRotation` (`KismetMathLibrary.MakeRotator` 0.0 0.0 (`self.zRotation`)))))

(fn `UserConstructionScript`)