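; BP_ICE is an ice weapon actor that sends a damage message to actors its Box overlaps, ignoring BP_Player3.
; A valid overlap sets HitFlag and calls the damage interface with a value of zero.
; Tick destroys the actor once HitFlag is set, or after a three-second Delay otherwise.
; DestroyFunc spawns a Niagara explosion at the Box and destroys the actor, but nothing here calls it.
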(event `self.ReceiveTick`
  (params (DeltaSeconds :type "Float (single-precision)"))
  (if (not (`self.HitFlag`))
    (`KismetSystemLibrary.Delay` 3.0))
  (`self.K2_DestroyActor`))

(event `self.Box.OnComponentBeginOverlap`
  (params (OverlappedComponent :type "PrimitiveComponent Object Reference") (OtherActor :type "Actor Object Reference") (OtherComp :type "PrimitiveComponent Object Reference") (OtherBodyIndex :type Integer) (bFromSweep :type Boolean) (SweepResult :type "HitResult Structure (by ref)"))
  (cast `/Game/Whisper/BP_Player3` OtherActor
    (:`CastFailed`
      (set `self.HitFlag` true)
      (message `/Game/Map/BPI_Battle.I_DamageEvent` OtherActor 0.0))))

(fn `DestroyFunc`
  (bind _box (`self.Box`))
  (`NiagaraFunctionLibrary.SpawnSystemAtLocation` "/Game/AdvancedMagicFX13/Particles/Niagara/NS_ky_explosion1.NS_ky_explosion1" (`SceneComponent.K2_GetComponentLocation` _box) (`SceneComponent.K2_GetComponentRotation` _box))
  (`self.K2_DestroyActor`))

(fn `UserConstructionScript`)